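; BP_DayNightSun is the sun actor for the day/night cycle, driven by the TimeOfDay subsystem.
; On BeginPlay it binds to the subsystem's sunrise and moonrise events, showing the root and its children at sunrise and hiding them at moonrise.
; Each tick it sets the directional light's relative rotation from the subsystem's sun rotation.
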(event Custom|OnMoonrise_Event
  (params (MoonPhase :type Float%20%28single-precision%29) (CurrentTime :type Time%20Of%20Day%20Time%20Structure%20%28by%20ref%29))
  (Rendering|SetVisibility (Variables|Default|GetDefaultSceneRoot) false true))

(event Custom|OnSunrise_Event
  (params (CurrentTime :type Time%20Of%20Day%20Time%20Structure%20%28by%20ref%29))
  (Rendering|SetVisibility (Variables|Default|GetDefaultSceneRoot) true true))

(event EventBeginPlay
  (Utilities|FlowControl|Sequence
    (:then_0
      (EventDispatchers|AssignOnSunrise (Class|TimeOfDayBlueprintLibrary|GetTimeOfDaySubsystem) (delegate Custom|OnSunrise_Event)))
    (:then_1
      (EventDispatchers|AssignOnMoonrise (Class|TimeOfDayBlueprintLibrary|GetTimeOfDaySubsystem) (delegate Custom|OnMoonrise_Event)))))

(event Collision|EventActorBeginOverlap
  (params (OtherActor :type Actor%20Object%20Reference)))

(event EventTick
  (params (DeltaSeconds :type Float%20%28single-precision%29))
  (Transformation|SetRelativeRotation (Variables|Default|GetDirectionalLight) (Class|TimeOfDaySubsystem|GetSunRotation (Class|TimeOfDayBlueprintLibrary|GetTimeOfDaySubsystem)) false false))

(fn ConstructionScript)