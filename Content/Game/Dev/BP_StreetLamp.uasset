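; BP_StreetLamp is a street lamp actor that switches its point light on and off with the in-game time of day.
; On BeginPlay it binds to the TimeOfDay subsystem's sunset, sunrise and hour-changed events.
; Sunset raises the light intensity and sunrise zeroes it.
; The hourly event also lights the lamp early at 17:00 during Winter.
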(event Custom|OnSunset_Event
  (params (CurrentTime :type Time%20Of%20Day%20Time%20Structure%20%28by%20ref%29))
  (Rendering|Components|Light|SetIntensity (Variables|Default|GetPointLight) 1.5e+04))

(event Custom|OnSunrise_Event
  (params (CurrentTime :type Time%20Of%20Day%20Time%20Structure%20%28by%20ref%29))
  (Rendering|Components|Light|SetIntensity (Variables|Default|GetPointLight) 0.0))

(event Custom|OnHourChanged_Event
  (params (CurrentTime :type Time%20Of%20Day%20Time%20Structure%20%28by%20ref%29))
  (if (and (== (.hour CurrentTime) 17) (Utilities|Enum|Equal(Enum) (.season CurrentTime) "Winter"))
    (Rendering|Components|Light|SetIntensity (Variables|Default|GetPointLight) 1.5e+04)))

(event EventBeginPlay
  (Utilities|FlowControl|Sequence
    (:then_0
      (EventDispatchers|AssignOnSunset (Class|TimeOfDayBlueprintLibrary|GetTimeOfDaySubsystem) (delegate Custom|OnSunset_Event)))
    (:then_1
      (EventDispatchers|AssignOnSunrise (Class|TimeOfDayBlueprintLibrary|GetTimeOfDaySubsystem) (delegate Custom|OnSunrise_Event)))
    (:then_2
      (EventDispatchers|AssignOnHourChanged (Class|TimeOfDayBlueprintLibrary|GetTimeOfDaySubsystem) (delegate Custom|OnHourChanged_Event)))))

(event Collision|EventActorBeginOverlap
  (params (OtherActor :type Actor%20Object%20Reference)))

(event EventTick
  (params (DeltaSeconds :type Float%20%28single-precision%29)))

(fn ConstructionScript)